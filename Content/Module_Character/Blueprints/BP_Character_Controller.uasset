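; Player controller Blueprint that toggles the main menu widget through an exit-button handler.
; If a menu exists, the handler removes all widgets, restores game-only input, hides the cursor and clears the reference.
; Otherwise it creates the Module Menu Main widget with ThirdPersonMap as its new-game level, initializes it, adds it to the viewport and focuses it in game-and-UI input mode.
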(event EventOnButtonExit
  ;[0.15 0.15 0.15 0.5] Q or ESC button Handler
  ;   - Create Menu | Exit from Menu
  ;   - Something Skip or Cancel
  ;   - Work only with Module Menu Main
  (Variables|Default|GetMenu_Main
    (:then
      (Viewport|RemoveAllWidgets)
      (Input|SetInputModeGameOnly self false)
      (Variables|Default|SetbShowMouseCursor self false)
      (Variables|Default|SetMenu_Main 0))
    (:else
      (bind _returnvalue (UserInterface|CreateWidget "/Game/Module_Menu/Widgets/WBP_Module_Menu_Main.WBP_Module_Menu_Main_C" self))
      (bind _output_get (Variables|Default|SetMenu_Main _returnvalue))
      (Class|AModuleMenuMain|CreateMenuMain _output_get true)
      (UserInterface|Viewport|AddtoViewport (Variables|Default|GetMenu_Main) 0)
      (Input|SetInputModeGameandUI self (Variables|Default|GetMenu_Main) "DoNotLock" false false))))

(fn ConstructionScript)